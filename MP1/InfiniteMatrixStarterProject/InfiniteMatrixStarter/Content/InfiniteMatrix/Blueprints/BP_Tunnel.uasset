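; BP_Tunnel is a tunnel segment with a rotating holed wall that the player must pass through.
; Randomize functions, not called here, pick one of four wall meshes and a spin speed, and may spawn a health pack or enemy short of the trigger.
; Reaching the trigger awards points, has TunnelSpawner spawn another tunnel, and destroys this one.
; Hitting the wall deducts points and health and shifts the player along X.
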(event `self.ReceiveTick`
  (params (DeltaSeconds :type "Float (single-precision)"))
  (`SceneComponent.K2_AddLocalRotation` (`self.WallMesh`) (`KismetMathLibrary.MakeRotator` (* DeltaSeconds (`self.RotateSpeed`))) false false))

(event `self.TriggerZone.OnComponentBeginOverlap`
  (params (OverlappedComponent :type "PrimitiveComponent Object Reference") (OtherActor :type "Actor Object Reference") (OtherComp :type "PrimitiveComponent Object Reference") (OtherBodyIndex :type Integer) (bFromSweep :type Boolean) (SweepResult :type "HitResult Structure (by ref)"))
  (bind _asbp_player (cast `/Game/InfiniteMatrix/Blueprints/BP_Player` OtherActor))
  (`/Game/InfiniteMatrix/Blueprints/BP_Player.ChangePoints` _asbp_player 100)
  (`/Game/InfiniteMatrix/Blueprints/BP_TunnelSpawner.SpawnTunnelAtSpawnPoint` (`self.TunnelSpawner`))
  (`self.K2_DestroyActor`))

(event `self.WallMesh.OnComponentHit`
  (params (HitComponent :type "PrimitiveComponent Object Reference") (OtherActor :type "Actor Object Reference") (OtherComp :type "PrimitiveComponent Object Reference") (NormalImpulse :type "Vector Structure") (Hit :type "HitResult Structure (by ref)"))
  (bind _asbp_player (cast `/Game/InfiniteMatrix/Blueprints/BP_Player` OtherActor))
  (`/Game/InfiniteMatrix/Blueprints/BP_Player.ChangePoints` _asbp_player -100)
  (`self.K2_AddActorWorldOffset` _asbp_player (100.0 0.0 0.0) false false)
  (`/Game/InfiniteMatrix/Blueprints/BP_Player.ChangeHealth` _asbp_player -1.0))

(fn `RandomizeEnemy`
  (bind _returnvalue_x (`KismetMathLibrary.BreakVector` (`SceneComponent.K2_GetComponentLocation` (`self.TriggerZone`))))
  (if (< (`KismetMathLibrary.RandomIntegerInRange` 0 9) 3)
    (`|SpawnActorFromClass` "/Game/InfiniteMatrix/Blueprints/Enemy.Enemy_C" (`KismetMathLibrary.MakeTransform` (`KismetMathLibrary.MakeVector` (- _returnvalue_x (`KismetMathLibrary.RandomFloatInRange` 800.0 1200.0)) (`KismetMathLibrary.RandomFloatInRange` -300.0 300.0) (`KismetMathLibrary.RandomFloatInRange` -200.0 200.0))) "Undefined" "MultiplyWithRoot" null null)))

(fn `RandomizeHealthpack`
  (bind _returnvalue_x (`KismetMathLibrary.BreakVector` (`SceneComponent.K2_GetComponentLocation` (`self.TriggerZone`))))
  (if (< (`KismetMathLibrary.RandomIntegerInRange` 0 9) 3)
    (bind _returnvalue (`|SpawnActorFromClass` "/Game/InfiniteMatrix/Blueprints/HealthPack.HealthPack_C" (`KismetMathLibrary.MakeTransform` (`KismetMathLibrary.MakeVector` (- _returnvalue_x (`KismetMathLibrary.RandomFloatInRange` 800.0 1200.0)) (`KismetMathLibrary.RandomFloatInRange` -300.0 300.0) (`KismetMathLibrary.RandomFloatInRange` -200.0 200.0))) "Undefined" "MultiplyWithRoot" null null))
    (set `self.HealthPack` _returnvalue)))

(fn `RandomizeWall`
  (`StaticMeshComponent.SetStaticMesh` (`self.WallMesh`) (select `int` (`KismetMathLibrary.RandomIntegerInRange` 0 3) :`0` "/Game/InfiniteMatrix/Meshes/SM_Hole_01.SM_Hole_01" :`1` "/Game/InfiniteMatrix/Meshes/SM_Hole_02.SM_Hole_02" :`2` "/Game/InfiniteMatrix/Meshes/SM_Hole_03.SM_Hole_03" :`3` "/Game/InfiniteMatrix/Meshes/SM_Hole_04.SM_Hole_04" :!type "StaticMesh Object Reference"))
  (set `self.RotateSpeed` (`KismetMathLibrary.RandomFloatInRange` -60.0 60.0)))

(fn `UserConstructionScript`)